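; Game mode for a local multiplayer King of Bombs match that runs last-player-standing rounds.
; On begin play it starts music and calls RestartLevel, which recreates local players at player starts named by index and gives each a UI widget.
; Tick labels dead players, announces the sole survivor as winner then reloads the level after a delay, and switches music once at least two players are dead.
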(event Custom|Restart%20Level
  (bind _returnvalue (Game|GetPlayerController 0))
  (Utilities|FlowControl|Sequence
    (:then_0
      (for _array_element (Variables|Default|GetPlayers)
        (Class|GameplayStatics|RemovePlayer _array_element true))
      (Utilities|Array|Clear (Variables|Default|GetPlayers)))
    (:then_1
      (for _index (range 0 4)
        (bind _returnvalue_2 (Class|GameplayStatics|CreatePlayer _index))
        (Class|GameModeBase|RestartPlayeratPlayerStart _returnvalue_2 (Class|GameModeBase|FindPlayerStart _returnvalue_2 (Utilities|String|ToString(Integer) _index)))))
    (:then_2
      (Class|GameModeBase|RestartPlayeratPlayerStart _returnvalue (Class|GameModeBase|FindPlayerStart _returnvalue "0")))
    (:then_3
      (bind _outactors (Actor|GetAllActorsOfClass "/Script/KingOfBombs.KingOfBombsCharacter"))
      (for _array_element_2 _outactors
        (bind _asplayer_controller (Utilities|Casting|CastToPlayerController (Pawn|GetController _array_element_2)))
        (Utilities|Array|Add (Variables|Default|GetPlayers) _asplayer_controller)))
    (:then_4
      (Utilities|FlowControl|Delay 0.2)
      (for _array_element_3 (Variables|Default|GetPlayers)
        (Utilities|IsValid _array_element_3
          (:Is%20Valid
            (bind _returnvalue_3 (UserInterface|CreateWidget "/Game/Blueprints/UI.UI_C" _array_element_3))
            (Variables|/Game/Blueprints/UI.UI_C|SetController _returnvalue_3 _array_element_3)
            (UserInterface|Viewport|AddtoPlayerScreen _returnvalue_3)
            (Utilities|IsValid (Pawn|GetControlledPawn _array_element_3)
              (:Is%20Valid
                (bind _askbplayer (Utilities|Casting|CastToKBPlayer (Pawn|GetControlledPawn _array_element_3)))
                (bind _asnew_blueprint (Utilities|Casting|CastToNewBlueprint _askbplayer))
                (Variables|/Game/Blueprints/NewBlueprint.NewBlueprint_C|SetUI _asnew_blueprint _returnvalue_3)))))))))

(event EventBeginPlay
  (Utilities|FlowControl|Sequence
    (:then_0
      (bind _returnvalue (Audio|SpawnSound2D "/Game/Sounds/BGM/GeneralPlay.GeneralPlay" 1.0 1.0 0.0 0))
      (Variables|Default|SetTargetAudio _returnvalue))
    (:then_1
      (CallFunction|RestartLevel))))

(event EventTick
  (params (DeltaSeconds :type Float%20%28single-precision%29))
  (Utilities|FlowControl|Sequence
    (:then_0
      (for _array_element (Variables|Default|GetPlayers)
        (Utilities|IsValid _array_element
          (:Is%20Valid
            (Utilities|IsValid (Pawn|GetControlledPawn _array_element)
              (:Is%20Valid
                (bind _askbplayer (Utilities|Casting|CastToKBPlayer (Pawn|GetControlledPawn _array_element)))
                (Variables|Default|SetAlive false)
                (if (Variables|/Script/KingOfBombs.KingOfBombsCharacter|GetDead _askbplayer)
                  (bind _asnew_blueprint (Utilities|Casting|CastToNewBlueprint _askbplayer))
                  (Rendering|Components|TextRender|SetText (Variables|/Game/Blueprints/UI.UI_C|GetTextBlock_0 (Variables|/Game/Blueprints/NewBlueprint.NewBlueprint_C|GetUI _asnew_blueprint)) "Dead")
                  (else
                    (for _array_element_2 (Variables|Default|GetPlayers)
                      (if (!= _array_element_2 _array_element)
                        (Utilities|IsValid (Pawn|GetControlledPawn _array_element_2)
                          (:Is%20Valid
                            (bind _askbplayer_2 (Utilities|Casting|CastToKBPlayer (Pawn|GetControlledPawn _array_element_2)))
                            (if (not (Variables|/Script/KingOfBombs.KingOfBombsCharacter|GetDead _askbplayer_2))
                              (Variables|Default|SetAlive true))))))
                    (if (not (Variables|Default|GetAlive))
                      (bind _askbplayer_3 (Utilities|Casting|CastToKBPlayer (Pawn|GetControlledPawn _array_element)))
                      (bind _asnew_blueprint_2 (Utilities|Casting|CastToNewBlueprint _askbplayer_3))
                      (Rendering|Components|TextRender|SetText (Variables|/Game/Blueprints/UI.UI_C|GetTextBlock_0 (Variables|/Game/Blueprints/NewBlueprint.NewBlueprint_C|GetUI _asnew_blueprint_2)) "you win")
                      (Utilities|FlowControl|Delay 2.0)
                      (CallFunction|RestartLevel)
                      (bind _returnvalue (Game|GetCurrentLevelName true))
                      (Game|OpenLevel(byName) (Utilities|String|StringToName _returnvalue)))))))))))
    (:then_1
      (Variables|Default|SetLeft 0))
    (:then_2
      (bind _outactors (Actor|GetAllActorsOfClass "/Script/KingOfBombs.KBPlayer"))
      (for _array_element_3 _outactors
        (if (Variables|/Script/KingOfBombs.KingOfBombsCharacter|GetDead _array_element_3)
          (bind _output_get (Variables|Default|SetLeft (+ (Variables|Default|GetLeft) 1)))
          (bind _output_get_2 (Variables|Default|SetChange%20Audio (>= _output_get 2)))
          (if _output_get_2
            (Utilities|FlowControl|DoOnce false
              (:Completed
                (Audio|PlaySound2D "/Game/Sounds/BGM/BGMTwo.BGMTwo" 1.0 1.0 0.0 0 0)
                (Audio|Components|Audio|Stop (Variables|Default|GetTargetAudio))))))))))

(fn ConstructionScript)